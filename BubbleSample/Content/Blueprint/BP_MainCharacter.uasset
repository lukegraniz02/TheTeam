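; BP_MainCharacter is the player character Blueprint, handling camera-relative movement through Enhanced Input.
; IA_Move drives movement input along the player camera manager's right and forward vectors.
; The same handler looks up BP_Camera on each trigger and passes both axis values to its OnPlayersMovementEvent.
; Nodes for adding the IM_Controls mapping context and switching the view target to BP_Camera are disconnected and never run.
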(event `self.ReceiveBeginPlay`)

(event `EnhancedInput|/Game/InputActions/IA_Move`
  (params (ActionValue :type "Vector2D Structure") (ElapsedSeconds :type "Float (double-precision)") (TriggeredSeconds :type "Float (double-precision)") (InputAction :type "InputAction Object Reference" :default "/Game/InputActions/IA_Move.IA_Move"))
  ;[0 0 0] Movement
  (:`Triggered`
    (set `self.Action Value X` ActionValue_X)
    (`self.AddMovementInput` (`self.GetActorRightVector` (`GameplayStatics.GetPlayerCameraManager` 0)) ActionValue_X)
    (`self.AddMovementInput` (`self.GetActorForwardVector` (`GameplayStatics.GetPlayerCameraManager` 0)) ActionValue_Y)
    (bind _returnvalue (`GameplayStatics.GetActorOfClass` "/Game/Blueprint/BP_Camera.BP_Camera_C"))
    (`/Game/Blueprint/BP_Camera.OnPlayersMovement_Event` _returnvalue ActionValue_X ActionValue_Y)))

(fn `UserConstructionScript`)