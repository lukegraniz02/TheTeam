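; BP_Player2 is a player Blueprint that registers an Enhanced Input mapping context when play begins.
; On BeginPlay it runs the parent logic, casts its controller to PlayerController and adds IM_Controls1 to that controller's Enhanced Input subsystem.
; Tick and overlap events are disabled and the construction script only calls its parent, so the graphs define no other behavior.
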(event `self.ReceiveBeginPlay`
  (`parent.ReceiveBeginPlay`)
  (bind _asplayer_controller (cast `PlayerController` (`self.GetController`)))
  (bind _returnvalue (pcsubsystem `EnhancedInputLocalPlayerSubsystem` _asplayer_controller))
  (`/Engine/EditorBlueprintResources/StandardMacros.IsValid` _returnvalue
    (:`Is Valid`
      (`EnhancedInputSubsystemInterface.AddMappingContext` _returnvalue "/Game/InputActions/IM_Controls1.IM_Controls1" 0 (struct)))))

(fn `UserConstructionScript`
  (`parent.UserConstructionScript`))