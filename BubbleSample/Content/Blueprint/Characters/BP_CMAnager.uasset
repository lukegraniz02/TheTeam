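; BP_CMAnager sets up Enhanced Input for two local players.
; On BeginPlay it adds IM_Controls to player controller 0 and IM_SecondPlayerControls to controller 1, both at the same priority.
; An unconnected loop over BP_MainCharacter actors, which would assign controller IDs and choose a mapping context by index, never runs.
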(event `self.ReceiveBeginPlay`
  (`EnhancedInputSubsystemInterface.AddMappingContext` (pcsubsystem `EnhancedInputLocalPlayerSubsystem` (`GameplayStatics.GetPlayerController` 0)) "/Game/InputActions/IM_Controls.IM_Controls" 0 (struct))
  (`EnhancedInputSubsystemInterface.AddMappingContext` (pcsubsystem `EnhancedInputLocalPlayerSubsystem` (`GameplayStatics.GetPlayerController` 1)) "/Game/InputActions/IM_SecondPlayerControls.IM_SecondPlayerControls" 0 (struct)))

(fn `UserConstructionScript`)