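; Player character for a bubble shooter where PlayerBubbleLife acts as health, shown in a Vite_giocatori widget.
; Moves relative to player 0's camera and notifies BP_Camera of movement input.
; Blow and suck shots spawn BP_PlayerBullets; blowing applies recoil to life, suck hits restore it, and overlapped bubble pickups add their size directly.
; ModifyLife disables the player outside life limits and runs a high-life countdown toward the still-empty WinCondition.
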(event `self.ReceiveBeginPlay`
  (bind _returnvalue (`|CreateWidget` "/Game/UI/UI/Vite_giocatori.Vite_giocatori_C"))
  (bind _output_get (set `self.UiWidget` _returnvalue))
  (`UserWidget.AddToViewport` _output_get 0))

(event `WinCondition`)

(event `self.ReceiveTick`
  (params (DeltaSeconds :type "Float (single-precision)"))
  (if (`self.Countdown`)
    (bind _output_get (set `self.Timer` (+ DeltaSeconds (`self.Timer`))))
    (`KismetSystemLibrary.PrintString` (`KismetStringLibrary.Conv_DoubleToString` _output_get))
    (if (> _output_get 10.0)
      (`self.WinCondition`))))

(event `EnhancedInput|/Game/InputActions/IA_Move`
  (params (ActionValue :type "Vector2D Structure") (ElapsedSeconds :type "Float (double-precision)") (TriggeredSeconds :type "Float (double-precision)") (InputAction :type "InputAction Object Reference" :default "/Game/InputActions/IA_Move.IA_Move"))
  ;[0 0 0] Movement
  (:`Triggered`
    (set `self.Action Value X` ActionValue_X)
    (`self.AddMovementInput` (`self.GetActorRightVector` (`GameplayStatics.GetPlayerCameraManager` 0)) ActionValue_X)
    (`self.AddMovementInput` (`self.GetActorForwardVector` (`GameplayStatics.GetPlayerCameraManager` 0)) ActionValue_Y)
    (bind _returnvalue (`GameplayStatics.GetActorOfClass` "/Game/Blueprint/BP_Camera.BP_Camera_C"))
    (`/Game/Blueprint/BP_Camera.OnPlayersMovement_Event` _returnvalue ActionValue_X ActionValue_Y)))

(event `EnhancedInput|/Game/InputActions/IA_Look`
  (params (ActionValue :type "Vector2D Structure") (ElapsedSeconds :type "Float (double-precision)") (TriggeredSeconds :type "Float (double-precision)") (InputAction :type "InputAction Object Reference" :default "/Game/InputActions/IA_Look.IA_Look"))
  (:`Triggered`
    (`self.AddControllerYawInput` ActionValue_X)
    (`self.AddControllerPitchInput` ActionValue_Y)))

(event `ModifyLife`
  (params (LifeChange :type "Float (double-precision)"))
  (set `self.Player Bubble Life` (+ (`self.Player Bubble Life`) LifeChange))
  (if (and (< (`self.Player Bubble Life`) (`self.MaxLife`)) (> (`self.Player Bubble Life`) (`self.MinLife`)))
    (`KismetSystemLibrary.PrintString` (`KismetStringLibrary.Conv_DoubleToString` (`self.Player Bubble Life`)))
    (if (> (`self.Player Bubble Life`) 90.0)
      (if (not (`self.Countdown`))
        (set `self.Countdown` true)
        (set `self.Timer` 0.0))
      (elif (`self.Countdown`)
        (set `self.Countdown` false)
        (set `self.Timer` 0.0)))
    (else
      (`KismetSystemLibrary.PrintString` "death")
      (`self.OnDeath`)))
  (`/Game/UI/UI/Vite_giocatori.GetPercent_0` (`self.UiWidget`)))

(event `OnDeath`
  (`self.DisablePlayer`))

(event `EnhancedInput|/Game/InputActions/IA_ShootBlow`
  (params (ActionValue :type Boolean) (ElapsedSeconds :type "Float (double-precision)") (TriggeredSeconds :type "Float (double-precision)") (InputAction :type "InputAction Object Reference" :default "/Game/InputActions/IA_ShootBlow.IA_ShootBlow"))
  (:`Started`
    (`self.ModifyLife` (`self.BlowRecoilDamage`))
    (`self.Shoot` (`self.BlowDamage`))))

(event `EnhancedInput|/Game/InputActions/IA_ShootSuck`
  (params (ActionValue :type Boolean) (ElapsedSeconds :type "Float (double-precision)") (TriggeredSeconds :type "Float (double-precision)") (InputAction :type "InputAction Object Reference" :default "/Game/InputActions/IA_ShootSuck.IA_ShootSuck"))
  (:`Started`
    (bind _bullet (`self.Shoot` (`self.SuckDamage`)))
    (add `/Game/Blueprint/Gun/BP_PlayerBullets.OnSuckHit` _bullet (delegate `GainLife`))))

(event `GainLife`
  (`self.ModifyLife` (`self.SuckGainedLife`)))

(event `self.CapsuleComponent.OnComponentBeginOverlap`
  (params (OverlappedComponent :type "PrimitiveComponent Object Reference") (OtherActor :type "Actor Object Reference") (OtherComp :type "PrimitiveComponent Object Reference") (OtherBodyIndex :type Integer) (bFromSweep :type Boolean) (SweepResult :type "HitResult Structure (by ref)"))
  (if (`KismetSystemLibrary.DoesImplementInterface` OtherActor "/Game/Interfaces/BPI_PickUpBubbles.BPI_PickUpBubbles_C")
    (`/Engine/EditorBlueprintResources/StandardMacros.DoOnce` false :!label _label
      (:`Completed`
        (bind _setbubblesizevalue (message `/Game/Interfaces/BPI_PickUpBubbles.GetBubbleSizeValue` OtherActor))
        (bind _output_get (set `self.Player Bubble Life` (+ (`self.Player Bubble Life`) _setbubblesizevalue)))
        (`KismetSystemLibrary.PrintString` (`KismetStringLibrary.Conv_DoubleToString` _output_get))
        (`KismetSystemLibrary.DelayUntilNextTick`)
        (`self.K2_DestroyActor` OtherActor)))))

(event `ResetDoOnce`
  (goto _label :!via `Reset`))

(event `self.CapsuleComponent.OnComponentEndOverlap`
  (params (OverlappedComponent :type "PrimitiveComponent Object Reference") (OtherActor :type "Actor Object Reference") (OtherComp :type "PrimitiveComponent Object Reference") (OtherBodyIndex :type Integer))
  (`self.ResetDoOnce`))

(fn `DisablePlayer`
  (`PrimitiveComponent.SetCollisionEnabled` (`self.CapsuleComponent`) "NoCollision")
  (`SceneComponent.SetHiddenInGame` (`self.StaticMesh`) true false)
  (`SceneComponent.SetHiddenInGame` (`self.CharacterMesh`) true false)
  (`self.DisableInput` null))

(fn `Shoot`
  (params (`BlowOrSuck?` :type "Float (double-precision)"))
  (returns (Bullet :type "/Game/Blueprint/Gun/BP_PlayerBullets Object Reference"))
  (locals (`Projectile Distance` :type "Float (double-precision)" :default 5000.0))
  (bind _arrow1 (`self.Arrow1`))
  (bind _returnvalue (`SceneComponent.K2_GetComponentLocation` _arrow1))
  (`KismetSystemLibrary.PrintString` (`KismetStringLibrary.Conv_VectorToString` _returnvalue))
  (bind _returnvalue_2 (`|SpawnActorFromClass` "/Game/Blueprint/Gun/BP_PlayerBullets.BP_PlayerBullets_C" (`KismetMathLibrary.MakeTransform` _returnvalue (`SceneComponent.K2_GetComponentRotation` _arrow1)) "Undefined" "MultiplyWithRoot" null self `BlowOrSuck?` null))
  (return _returnvalue_2))

(fn `UserConstructionScript`)