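; BP_Player1 is the first player's character, with blow and suck shots that trade life.
; On BeginPlay it adds the IM_Controls Enhanced Input mapping context to player controller 0.
; Blow input applies recoil through ModifyLife and fires Shoot with blow damage.
; Suck input fires Shoot with suck damage and binds the result's OnSuckHit to a life gain, though both shots pass IsBlow as false.
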(event `self.ReceiveBeginPlay`
  (bind _returnvalue (pcsubsystem `EnhancedInputLocalPlayerSubsystem` (`GameplayStatics.GetPlayerController` 0)))
  (`parent.ReceiveBeginPlay`)
  (`/Engine/EditorBlueprintResources/StandardMacros.IsValid` _returnvalue
    (:`Is Valid`
      (`EnhancedInputSubsystemInterface.AddMappingContext` _returnvalue "/Game/InputActions/IM_Controls.IM_Controls" 0 (struct)))))

(event `EnhancedInput|/Game/InputActions/IA_ShootBlow`
  (params (ActionValue :type Boolean) (ElapsedSeconds :type "Float (double-precision)") (TriggeredSeconds :type "Float (double-precision)") (InputAction :type "InputAction Object Reference" :default "/Game/InputActions/IA_ShootBlow.IA_ShootBlow"))
  (:`Started`
    (`self.ModifyLife` (`self.BlowRecoilDamage_0`))
    (`self.Shoot` (`self.BlowDamage_0`))))

(event `EnhancedInput|/Game/InputActions/IA_ShootSuck`
  (params (ActionValue :type Boolean) (ElapsedSeconds :type "Float (double-precision)") (TriggeredSeconds :type "Float (double-precision)") (InputAction :type "InputAction Object Reference" :default "/Game/InputActions/IA_ShootSuck.IA_ShootSuck"))
  (:`Started`
    (bind _bullet (`self.Shoot` (`self.SuckDamage_0`)))
    (add `/Game/Blueprint/Gun/BP_PlayerBullets.OnSuckHit` _bullet (delegate `GainLife`))))

(event `GainLife`
  (`self.ModifyLife` (`self.SuckGainedLife_0`)))

(fn `UserConstructionScript`
  (`parent.UserConstructionScript`))