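; Shared camera actor that becomes player 0's view target at BeginPlay and frames BP_Player1 and BP_Player2.
; Each Tick, SpringArm1 sits on Player1, yawed along the line between players at half their distance, putting its end at their midpoint.
; A second spring arm scales its length with player separation above a minimum and lerps pitch over a normalized distance range, with a configurable relative yaw.
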(event `self.ReceiveBeginPlay`
  (`PlayerController.SetViewTargetWithBlend` (`GameplayStatics.GetPlayerController` 0) self 0.0 "VTBlend_Linear" 0.0 false))

(event `OnPlayersMovement_Event`
  (params (MovingOnXAxis :type "Float (double-precision)") (MovingOnYAxis :type "Float (double-precision)")))

(event `self.ReceiveTick`
  (params (DeltaSeconds :type "Float (single-precision)"))
  (bind _springarm (`self.SpringArm`))
  (bind _returnvalue (`GameplayStatics.GetActorOfClass` "/Game/Blueprint/Characters/BP_Player1.BP_Player1_C"))
  (bind _returnvalue_2 (`self.K2_GetActorLocation` _returnvalue))
  (`SceneComponent.K2_SetWorldLocation` (`self.SpringArm1`) _returnvalue_2 false false)
  (bind _returnvalue_3 (`GameplayStatics.GetActorOfClass` "/Game/Blueprint/Characters/BP_Player2.BP_Player2_C"))
  (bind _returnvalue_4 (`self.K2_GetActorLocation` _returnvalue_3))
  (bind (_returnvalue_roll _returnvalue_pitch _returnvalue_yaw) (`KismetMathLibrary.BreakRotator` (`KismetMathLibrary.FindLookAtRotation` _returnvalue_4 _returnvalue_2)))
  (`SceneComponent.K2_SetWorldRotation` (`self.SpringArm1`) (`KismetMathLibrary.MakeRotator` _returnvalue_roll 0.0 _returnvalue_yaw) false false)
  (bind _returnvalue_5 (/ (`KismetMathLibrary.Vector_Distance` _returnvalue_4 _returnvalue_2) 2.0))
  (set `SpringArmComponent.TargetArmLength` _returnvalue_5 (`self.SpringArm1`))
  (set `SpringArmComponent.TargetArmLength` (`KismetMathLibrary.FMax` (* _returnvalue_5 1.5) (`self.MinDistanceCamAdjustmen`)) _springarm)
  (`SceneComponent.K2_SetRelativeRotation` _springarm (`KismetMathLibrary.MakeRotator` 0.0 (`KismetMathLibrary.Lerp` (`self.Min Lerp`) (`self.Max Lerp`) (`KismetMathLibrary.FClamp` (`KismetMathLibrary.NormalizeToRange` _returnvalue_5 (`self.Normalize Range Min`) (`self.Normalize Range Max`)))) (`self.NewAttachedSpringArmYawRotation`)) false false))

(fn `UserConstructionScript`)